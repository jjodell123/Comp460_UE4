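; Lobby game mode that tracks joining players, syncs map settings and player lists to each LobbyPC, and server-travels to the selected map.
; PostLogin initializes each controller and possesses a base character at a random PlayerStart; joins and leaves trigger EveryoneUpdate.
; EveryoneUpdate rebuilds the roster, copies it to GameInfoInstance and flags start readiness by character class.
; SetupTeams alternates two teams; kick and character swap are empty stubs.
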(event Custom|SwapCharacter
  (params (PlayerController :type Player%20Controller%20Object%20Reference) (CharacterClass :type Character%20Class%20Reference) (ChangedStatus :type Boolean)))

(event Custom|EveryoneUpdate
  (bind _allplayercontrollers (Variables|ServerSettings|GetAllPlayerControllers))
  (bind _connectedplayers (Variables|ServerSettings|GetConnectedPlayers))
  ;[1 1 1] Updates connected players' lobby info
  (bind _output_get (Variables|ServerSettings|SetCurrentPlayers (Utilities|Array|Length (Variables|ServerSettings|GetAllPlayerControllers))))
  (if (> _output_get 0)
    (Utilities|Array|Clear (Variables|ServerSettings|GetConnectedPlayers))
    (for _array_element _allplayercontrollers
      (bind _aslobby_pc (Utilities|Casting|CastToLobbyPC _array_element))
      (Utilities|Array|Add (Variables|ServerSettings|GetConnectedPlayers) (Variables|/Game/Blueprints/Lobby/LobbyPC.LobbyPC_C|GetPlayerSettings _aslobby_pc))
      (Default|UpdateNumPlayers _aslobby_pc (Variables|ServerSettings|GetCurrentPlayers) (Variables|ServerSettings|GetMaxPlayers)))
    (for _array_element_2 _allplayercontrollers
      (bind _aslobby_pc_2 (Utilities|Casting|CastToLobbyPC _array_element_2))
      (Default|AddPlayerInfo _aslobby_pc_2 _connectedplayers)
      (Variables|/Game/Blueprints/AllLevels/GameInfoInstance.GameInfoInstance_C|SetAllPlayerInfos (.AsGame%20Info%20Instance (Utilities|Casting|CastToGameInfoInstance (Game|GetGameInstance))) _connectedplayers)
      (CallFunction|AddtoKickList))
    (bind _array_element_3 (Utilities|Array|ForEachLoopwithBreak (Variables|ServerSettings|GetConnectedPlayers))
      (:LoopBody
        (if (== (.PlayerCharacterClass (Utilities|Struct|BreakPlayerInfo _array_element_3)) "/Script/Comp460_UE4.PlayerCharacter")
          (Variables|ServerSettings|SetCanWeStart? false)
          (CallFunction|CannotStart)
          (else
            (Variables|ServerSettings|SetCanWeStart? true)))))))

(event Custom|LaunchGame
  ;[1 1 1] Launches the map
  (switch int (Variables|ServerSettings|GetGM_MapID)
    (:0
      (Development|ExecuteConsoleCommand "servertravel Demo" (Game|GetPlayerController 0)))))

(event Custom|RespawnPlayer
  (params (PlayerController :type Player%20Controller%20Object%20Reference))
  (bind _spawnpoints (Variables|ServerSettings|GetSpawnPoints))
  ;[1 1 1] Spawn player as base character and tell everyone to update lobby
  (Utilities|IsValid (Pawn|GetControlledPawn PlayerController)
    (:Is%20Valid
      (Actor|DestroyActor))
    (:Is%20Not%20Valid
      _))
  (bind _returnvalue (Game|SpawnActorfromClass "/Script/Comp460_UE4.PlayerCharacter" (Transformation|GetActorTransform (Utilities|Array|Get(acopy) _spawnpoints (Math|Random|RandomIntegerinRange 0 (- (Utilities|Array|Length _spawnpoints) 1)))) "Undefined" 0 0))
  (Pawn|Possess PlayerController _returnvalue)
  (CallFunction|EveryoneUpdate))

(event Custom|AddToKickList)

(event Custom|CannotStart
  ;[1 1 1] Updates connected players' lobby info
  (Utilities|Array|ForEachLoopwithBreak (Variables|ServerSettings|GetConnectedPlayers)) ; enters at Break
)

(event Custom|ServerUpdateGameSettings
  (params (MapImage :type Texture%202D%20Object%20Reference) (MapName :type Text) (MapTime :type Text) (MapID :type Integer))
  ;[1 1 1] When server makes changes, tell clients to update their info
  (Variables|ServerSettings|SetGameModeMapImage MapImage)
  (Variables|ServerSettings|SetGameModeMapName MapName)
  (Variables|ServerSettings|SetGameModeMapTime MapTime)
  (Variables|ServerSettings|SetGM_MapID MapID)
  (for _array_element (Variables|ServerSettings|GetAllPlayerControllers)
    (bind _aslobby_pc (Utilities|Casting|CastToLobbyPC _array_element))
    (Default|UpdateLobbySettings _aslobby_pc (Variables|ServerSettings|GetGameModeMapImage) (Variables|ServerSettings|GetGameModeMapName) (Variables|ServerSettings|GetGameModeMapTime))))

(event Custom|SetupTeams
  (bind _returnvalue (Game|GetGameInstance))
  (bind _connectedplayers (Variables|ServerSettings|GetConnectedPlayers))
  (bind _returnvalue_2 (Utilities|Array|Length _connectedplayers))
  (bind _asgame_info_instance (Utilities|Casting|CastToGameInfoInstance _returnvalue))
  (bind _allplayerinfos (Variables|/Game/Blueprints/AllLevels/GameInfoInstance.GameInfoInstance_C|GetAllPlayerInfos _asgame_info_instance))
  ;[1 1 1] Sets team number for all players
  (Variables|/Game/Blueprints/AllLevels/GameInfoInstance.GameInfoInstance_C|SetTotalPlayers (.AsGame%20Info%20Instance (Utilities|Casting|CastToGameInfoInstance (Game|GetGameInstance))) _returnvalue_2)
  (for _index (range 0 (- _returnvalue_2 1))
    (Variables|Default|SetTempInfo (Utilities|Array|Get(acopy) (Variables|ServerSettings|GetConnectedPlayers) _index))
    (bind _structout (Utilities|Struct|SetmembersinPlayerInfo (Utilities|Array|Get(acopy) (Variables|ServerSettings|GetConnectedPlayers) _index) (+ (Math|Integer|%(Integer) _index 2) 1)))
    (Default|SetTeam (.AsLobby%20PC (Utilities|Casting|CastToLobbyPC (Utilities|Array|Get(acopy) (Variables|ServerSettings|GetAllPlayerControllers) _index))) (+ (Math|Integer|%(Integer) _index 2) 1))
    (Utilities|Array|SetArrayElem _allplayerinfos (Utilities|Array|FindItem _allplayerinfos (Variables|Default|GetTempInfo)) _structout)))

(event Custom|PlayerLeave
  (params (Controller :type Player%20Controller%20Object%20Reference))
  (Utilities|Array|RemoveItem (Variables|ServerSettings|GetAllPlayerControllers) Controller)
  (CallFunction|EveryoneUpdate))

(event EventPostLogin
  (params (NewPlayer :type Player%20Controller%20Object%20Reference))
  ;[1 1 1] Initial setup, occurs on event post login. Handles lobby setup
  (Networking|SwitchHasAuthority
    (:Authority
      (Utilities|Array|Add (Variables|ServerSettings|GetAllPlayerControllers) NewPlayer)
      (Utilities|Array|Add (Variables|/Game/Blueprints/AllLevels/GameInfoInstance.GameInfoInstance_C|GetAllPlayerControllers (.AsGame%20Info%20Instance (Utilities|Casting|CastToGameInfoInstance (Game|GetGameInstance)))) NewPlayer)
      (bind _outactors (Actor|GetAllActorsOfClass "/Script/Engine.PlayerStart"))
      (Variables|ServerSettings|SetSpawnPoints _outactors)
      (bind _asgame_info_instance (Utilities|Casting|CastToGameInfoInstance (Game|GetGameInstance)))
      (Variables|ServerSettings|SetServerName (Variables|/Game/Blueprints/AllLevels/GameInfoInstance.GameInfoInstance_C|GetServerName _asgame_info_instance))
      (Variables|ServerSettings|SetMaxPlayers (Variables|/Game/Blueprints/AllLevels/GameInfoInstance.GameInfoInstance_C|GetMaxPlayers _asgame_info_instance))
      (bind _aslobby_pc (Utilities|Casting|CastToLobbyPC NewPlayer))
      (Default|InitialSetup _aslobby_pc)
      (Default|SetupLobbyMenu _aslobby_pc (Variables|ServerSettings|GetServerName))
      (Default|UpdateLobbySettings _aslobby_pc (Variables|ServerSettings|GetGameModeMapImage) (Variables|ServerSettings|GetGameModeMapName) (Variables|ServerSettings|GetGameModeMapTime))
      (CallFunction|RespawnPlayer NewPlayer))))

(fn ConstructionScript)