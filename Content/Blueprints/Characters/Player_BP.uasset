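; Player character for a two-team shooter, handling player info, bullet hits, death and the end of a match.
; On possession it loads PlayerInfo from the game instance, which also drives the HUD, pause menu and win/lose screens.
; Overlapping projectiles from the opposing team, identified by actor tags, reduce health.
; Passthrough events forward kills, respawns and match results to Lockdown_Play_GameMode_BP, intended as server calls.
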(event Custom|GameWon
  ;[1 1 1] Handles game won and lost
  (Default|ShowWinScreen (Variables|Default|GetGameInstanceRef))
  (CallFunction|SignalFinishedEnding))

(event Custom|HandleHit
  (params (Other%20Actor :type Actor%20Object%20Reference))
  (bind _returnvalue (Game|GetInstigator Other%20Actor))
  (bind _self self)
  ;[1 1 1] Handles player getting shot
  (if (or (and (Actor|ActorHasTag _returnvalue "Team1") (Actor|ActorHasTag _self "Team2")) (and (Actor|ActorHasTag _returnvalue "Team2") (Actor|ActorHasTag _self "Team1")))
    (bind _output_get (Variables|Default|SetPlayerHealth (- (Variables|Default|GetPlayerHealth) (Variables|/Script/Comp460_UE4.MyProjectile|Getdamage (.AsMy%20Projectile%20BP (Utilities|Casting|CastToMyProjectile_BP Other%20Actor))))))
    (Default|UpdatePlayerHealth (Variables|Default|GetGameInstanceRef) _output_get)
    (CallFunction|DestroyServerActorPassthrough Other%20Actor)
    (CallFunction|CheckDead)))

(event Custom|CheckController
  (params (Controller :type Player%20Controller%20Object%20Reference))
  ;[1 1 1] Checks if the controllers match and sends results to the server if they do
  (CallFunction|ServerRun (Variables|PlayerSettings|GetPlayerInfo) (.AsPlayer%20Controller (Utilities|Casting|CastToPlayerController (Pawn|GetController)))))

(event Custom|ServerRun
  (params (Info :type Player%20Info%20Structure) (Controller :type Player%20Controller%20Object%20Reference))
  ;[1 1 1] Sends info and controller to the server
  (bind _aslockdown_play_game_mode_bp (Utilities|Casting|CastToLockdown_Play_GameMode_BP (Game|GetGameMode)))
  (Default|SavePlayerInfo _aslockdown_play_game_mode_bp Info Controller))

(event Custom|PlayerKilledPassthrough
  (params (TeamOfPlayerKilled :type Integer))
  ;[1 1 1] Sends player killed notice to the server
  (bind _aslockdown_play_game_mode_bp (Utilities|Casting|CastToLockdown_Play_GameMode_BP (Game|GetGameMode)))
  (Default|PlayerKilled _aslockdown_play_game_mode_bp TeamOfPlayerKilled))

(event Custom|SignalFinishedEnding
  ;[1 1 1] Adds a delay before sending players back to main menu
  (Utilities|FlowControl|Delay 3.0)
  (bind _aslockdown_play_game_mode_bp (Utilities|Casting|CastToLockdown_Play_GameMode_BP (Game|GetGameMode)))
  (Default|SignalGameEndedAcknowledged _aslockdown_play_game_mode_bp))

(event Custom|EndGame
  (bind _gameinstanceref (Variables|Default|GetGameInstanceRef))
  ;[1 1 1] Ends the game
  (Default|RemoveAllWidgets _gameinstanceref)
  (Default|RemovePlayerUI _gameinstanceref)
  (bind _structout (Utilities|Struct|SetmembersinPlayerInfo (Variables|PlayerSettings|GetPlayerInfo) 0))
  (Variables|PlayerSettings|SetPlayerInfo _structout)
  (Game|OpenLevel(byName) "MainMenu"))

(event Custom|GameLost
  ;[1 1 1] Handles game won and lost
  (Default|ShowLoseScreen (Variables|Default|GetGameInstanceRef))
  (CallFunction|SignalFinishedEnding))

(event Custom|CheckDead
  ;[1 1 1] Checks if player died, if they did handles death
  (if (<= (Variables|Default|GetPlayerHealth) 0)
    (Variables|Default|SetisDead true)
    (CallFunction|PlayerKilledPassthrough (.TeamNumber (Utilities|Struct|BreakPlayerInfo (Variables|PlayerSettings|GetPlayerInfo))))
    (Default|UpdatePlayerHealth (Variables|Default|GetGameInstanceRef) 100)
    (CallFunction|RespawnPassthrough (Game|GetPlayerController 0))))

(event Custom|SendGameOver
  (params (Winning%20Team :type Integer))
  ;[1 1 1] Ends the game
  (bind _aslockdown_play_game_mode_bp (Utilities|Casting|CastToLockdown_Play_GameMode_BP (Game|GetGameMode)))
  (Default|WinGame _aslockdown_play_game_mode_bp Winning%20Team))

(event Custom|DestroyServerActorPassthrough
  (params (ToDestroy :type Actor%20Object%20Reference))
  ;[1 1 1] Destroys actor on server
  (Actor|DestroyActor ToDestroy))

(event Custom|RespawnPassthrough
  (params (Controller :type Player%20Controller%20Object%20Reference))
  ;[1 1 1] Sends respawn notice to the server
  (bind _aslockdown_play_game_mode_bp (Utilities|Casting|CastToLockdown_Play_GameMode_BP (Game|GetGameMode)))
  (Default|RespawnPlayer _aslockdown_play_game_mode_bp Controller))

(event Custom|PrintHere
  (bind _playerinfo (Variables|PlayerSettings|GetPlayerInfo))
  (bind (_playername _playerimage _playercharacter _playercharacterimage _playerstatus _teamnumber) (Utilities|Struct|BreakPlayerInfo _playerinfo))
  ;[1 1 1] Debugging class to print the player info
  (Development|PrintString (Utilities|String|Append "Printing client " (Utilities|String|ToString(Text) _playername) " from team " (Utilities|String|ToString(Integer) _teamnumber)) true true "(R=0.000000,G=0.660000,B=1.000000,A=1.000000)" 2e+01))

(event Custom|LoadPlayerInfo
  ;[1 1 1] Loads player info
  (bind _asgame_info_instance (Utilities|Casting|CastToGameInfoInstance (Game|GetGameInstance)))
  (bind _output_get (Variables|Default|SetGameInstanceRef _asgame_info_instance))
  (Utilities|Struct|SetmembersinPlayerInfo (Variables|/Game/Blueprints/AllLevels/GameInfoInstance.GameInfoInstance_C|GetPlayerInfo _output_get) self)
  (bind _output_get_2 (Variables|PlayerSettings|SetPlayerInfo (Variables|/Game/Blueprints/AllLevels/GameInfoInstance.GameInfoInstance_C|GetPlayerInfo _output_get)))
  (Variables|/Game/Blueprints/AllLevels/GameInfoInstance.GameInfoInstance_C|SetPlayerInfo _asgame_info_instance _output_get_2)
  (if (>= (.TeamNumber (Utilities|Struct|BreakPlayerInfo _output_get_2)) 1)
    (Default|ShowPlayerUI _asgame_info_instance)
    (Default|SetupUIColors _asgame_info_instance (.TeamNumber (Utilities|Struct|BreakPlayerInfo _output_get_2)))))

(event Custom|AddTeamPoint
  (params (TeamOneKills :type Integer) (TeamTwoKills :type Integer))
  (bind _gameinstanceref (Variables|Default|GetGameInstanceRef))
  ;[1 1 1] Adds point to UI
  (if (== 1 (.TeamNumber (Utilities|Struct|BreakPlayerInfo (Variables|PlayerSettings|GetPlayerInfo))))
    (Default|UpdateTeamUI _gameinstanceref TeamOneKills TeamTwoKills)
    (else
      (Default|UpdateTeamUI _gameinstanceref TeamTwoKills TeamOneKills))))

(event Collision|EventActorBeginOverlap
  (params (OtherActor :type Actor%20Object%20Reference))
  ;[1 1 1] Handles player getting shot
  (if (not (== OtherActor (Variables|Default|GetPreviousBullet)))
    (Variables|Default|SetPreviousBullet OtherActor)
    (CallFunction|HandleHit OtherActor)))

(event EventPossessed
  (params (NewController :type Controller%20Object%20Reference))
  ;[1 1 1] Handles Event possesed
  (if (Utilities|Text|TextIsEmpty (.PlayerName (Utilities|Struct|BreakPlayerInfo (Variables|PlayerSettings|GetPlayerInfo))))
    (CallFunction|LoadPlayerInfo)))

(event Input|KeyboardEvents|Escape
  (params (Key :type Key%20Structure))
  (bind _gameinstanceref (Variables|Default|GetGameInstanceRef))
  (:Released
    (if (Variables|PlayerSettings|GetIsPaused)
      (Default|HidePauseMenu _gameinstanceref)
      (Variables|PlayerSettings|SetIsPaused false)
      (else
        (Default|ShowPauseMenu _gameinstanceref)
        (Variables|PlayerSettings|SetIsPaused true)))))

(fn ConstructionScript)