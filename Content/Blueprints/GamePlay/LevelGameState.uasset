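; LevelGameState is a level game state Blueprint that collects player character references in a PlayerCharacters array.
; The PassThrough and PassBack events each append the supplied character, with PassBack also printing a debug string containing its player name.
; A PrintHere call on the stored character is never executed, and BeginPlay and the construction script are empty.
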(event Custom|PassThrough
  (params (PlayerCharacter :type Player%20BP%20Object%20Reference))
  (bind _returnvalue (Utilities|Array|Add (Variables|Default|GetPlayerCharacters) PlayerCharacter)))

(event Custom|PassBack
  (params (PlayerCharacter :type Player%20BP%20Object%20Reference))
  (Utilities|Array|Add (Variables|Default|GetPlayerCharacters) PlayerCharacter)
  (Development|PrintString (Utilities|String|Append "EEEEEEEEEEEE" (Utilities|String|ToString(Text) (.PlayerName (Utilities|Struct|BreakPlayerInfo (Variables|/Game/Blueprints/Characters/Player_BP.Player_BP_C|GetPlayerInfo PlayerCharacter))))) true true "(R=0.000000,G=0.660000,B=1.000000,A=1.000000)" 2e+01))

(event EventBeginPlay)

(fn ConstructionScript)