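; Game mode for a two-team Lockdown match, covering player spawning, team scoring, victory and session teardown.
; On authority, joining players alternate between team pawn classes at random PlayerStarts.
; Saved controller-to-info map entries drive respawns with each player's character class, and kills update every pawn's score until a team reaches five and win/loss events fire.
; End acknowledgement notifies pawns, clears match state and destroys the session.
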(event Custom|DestroyServerActor
  (params (ToDestroy :type Actor%20Object%20Reference))
  ;[1 1 1] Destroys actor
  (Actor|DestroyActor ToDestroy))

(event Custom|PlayerKilled
  (params (Team :type Integer))
  ;[1 1 1] Sends out notice when the player is killed
  (if (== Team 2)
    (bind _output_get (Variables|GameSettings|SetTeamOneKills (+ (Variables|GameSettings|GetTeamOneKills) 1)))
    (else
      (bind _output_get_2 (Variables|GameSettings|SetTeamTwoKills (+ (Variables|GameSettings|GetTeamTwoKills) 1)))))
  (bind _keys (Utilities|Map|Keys (Variables|ServerSettings|GetAllPlayerControllers)))
  (for _array_element _keys
    (Default|AddTeamPoint (.AsPlayer%20BP (Utilities|Casting|CastToPlayer_BP (Pawn|GetControlledPawn _array_element))) _output_get _output_get_2))
  ;;[1 1 1] Checks if someone should win
  (if (>= (Variables|GameSettings|GetTeamOneKills) 5)
    (CallFunction|WinGame 1)
    (elif (>= (Variables|GameSettings|GetTeamTwoKills) 5)
      (CallFunction|WinGame 2))))

(event Custom|RespawnPlayer
  (params (Controller :type Player%20Controller%20Object%20Reference))
  (bind _returnvalue (Pawn|GetControlledPawn Controller))
  (bind _spawnpoints (Variables|ServerSettings|GetSpawnPoints))
  ;[1 1 1] Respawns the player with correct info at a spawn point
  (Utilities|IsValid _returnvalue
    (:Is%20Valid
      (Actor|DestroyActor _returnvalue)
      (bind _returnvalue_2 (Game|SpawnActorfromClass (.PlayerCharacterClass (Utilities|Struct|BreakPlayerInfo (.Value (Utilities|Map|Find (Variables|ServerSettings|GetAllPlayerControllers) Controller)))) (Transformation|GetActorTransform (Utilities|Array|Get(acopy) _spawnpoints (Math|Random|RandomIntegerinRange 0 (- (Utilities|Array|Length _spawnpoints) 1)))) "Undefined" 0 0))
      (Pawn|Possess Controller _returnvalue_2))))

(event Custom|WinGame
  (params (Team :type Integer))
  (bind _allplayercontrollers (Variables|ServerSettings|GetAllPlayerControllers))
  ;[1 1 1] Handles game win events
  (bind _keys (Utilities|Map|Keys _allplayercontrollers))
  (for _array_element _keys
    (if (== Team (.TeamNumber (Utilities|Struct|BreakPlayerInfo (.Value (Utilities|Map|Find _allplayercontrollers _array_element)))))
      (Default|GameWon (.AsPlayer%20BP (Utilities|Casting|CastToPlayer_BP (Pawn|GetControlledPawn _array_element))))
      (else
        (Default|GameLost (.AsPlayer%20BP (Utilities|Casting|CastToPlayer_BP (Pawn|GetControlledPawn _array_element))))))))

(event Custom|SignalGameEndedAcknowledged
  ;[1 1 1] Resets the game
  (bind _keys (Utilities|Map|Keys (Variables|ServerSettings|GetAllPlayerControllers)))
  (for (_array_element _array_index) _keys
    (Default|EndGame (.AsPlayer%20BP (Utilities|Casting|CastToPlayer_BP (Pawn|GetControlledPawn _array_element)))))
  (Variables|GameSettings|SetTeamOneKills 0)
  (Variables|GameSettings|SetTeamTwoKills 0)
  (Variables|ServerSettings|SetTotalPlayers 0)
  (Variables|ServerSettings|SetLoadedPlayers 0)
  (Variables|GameSettings|SetFinishedEnding 0)
  (Utilities|Map|Clear (Variables|ServerSettings|GetAllPlayerControllers))
  (Utilities|Array|Clear (Variables|ServerSettings|GetAllCharacters))
  (Utilities|Array|Clear (Variables|ServerSettings|GetAllPlayerInfos))
  (Utilities|Array|Clear (Variables|ServerSettings|GetSpawnPoints))
  (|DestroySession (Game|GetPlayerController 0)))

(event Custom|SavePlayerInfo
  (params (Info :type Player%20Info%20Structure) (Controller :type Player%20Controller%20Object%20Reference))
  ;[1 1 1] Saves Player info and controller to gamemode
  (Utilities|Map|Add (Variables|ServerSettings|GetAllPlayerControllers) Controller Info)
  (bind _asplayer_bp (Utilities|Casting|CastToPlayer_BP (Pawn|GetControlledPawn Controller)))
  (CallFunction|RespawnPlayer Controller))

(event EventHandleStartingNewPlayer
  (params (NewPlayer :type Player%20Controller%20Object%20Reference))
  ;[1 1 1] Handles player joining
  (Networking|SwitchHasAuthority
    (:Authority
      (if (== (Variables|ServerSettings|GetTotalPlayers) 0)
        (bind _outactors (Actor|GetAllActorsOfClass "/Script/Engine.PlayerStart"))
        (bind _output_get (Variables|ServerSettings|SetSpawnPoints _outactors))
        (Variables|ServerSettings|SetTotalPlayers (Variables|/Game/Blueprints/AllLevels/GameInfoInstance.GameInfoInstance_C|GetTotalPlayers (.AsGame%20Info%20Instance (Utilities|Casting|CastToGameInfoInstance (Game|GetGameInstance))))))
      (bind _output_get_2 (Variables|ServerSettings|SetLoadedPlayers (+ (Variables|ServerSettings|GetLoadedPlayers) 1)))
      (if (== (Math|Integer|%(Integer) _output_get_2 2) 0)
        (bind _returnvalue (Game|SpawnActorfromClass "/Game/Blueprints/Characters/Team2_Player.Team2_Player_C" (Transformation|GetActorTransform (.OutItem (Utilities|Array|Random _output_get))) "Undefined" NewPlayer 0))
        (Pawn|Possess NewPlayer _returnvalue)
        (Default|CheckController _returnvalue NewPlayer)
        (else
          (bind _returnvalue_2 (Game|SpawnActorfromClass "/Game/Blueprints/Characters/Team1_Player.Team1_Player_C" (Transformation|GetActorTransform (.OutItem (Utilities|Array|Random _output_get))) "Undefined" NewPlayer 0))
          (Pawn|Possess NewPlayer _returnvalue_2)
          (Default|CheckController _returnvalue_2 NewPlayer))))))

(fn ConstructionScript)